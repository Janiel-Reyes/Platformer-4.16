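; Weapon actor Blueprint that stores lethality, damage, ammo and range, set through a Stats event.
; Equip/Unequip mirrors the player ThirdPersonCharacter's LockedOn flag, toggling Equip and the actor's input.
; Firing_Gun uses a DoOnce, reset when Fired is false, to spend one round per press while equipped and print the remaining ammo.
; Firing only decrements ammo; no hit or damage logic is present.
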(event Custom|Equip/Unequip
  (bind _returnvalue (Game|GetPlayerController 0))
  ;[1 1 1] Process loss here
  (bind _asthird_person_character (Utilities|Casting|CastToThirdPersonCharacter (Game|GetPlayerCharacter 0)))
  (if (Variables|/Game/ThirdPersonBP/Blueprints/ThirdPersonCharacter.ThirdPersonCharacter_C|GetLockedOn _asthird_person_character)
    (Variables|Default|SetEquip true)
    (Input|EnableInput _returnvalue)
    (else
      (Variables|Default|SetEquip false)
      (Input|DisableInput _returnvalue))))

(event Custom|Firing_Gun
  (if (Variables|Default|GetEquip)
    (if (Variables|Default|GetFired)
      (if (not (== (Variables|Default|GetAmmo) 0.0))
        (Utilities|FlowControl|DoOnce false :!label _label
          (:Completed
            (bind _output_get (Variables|Default|SetAmmo (- (Variables|Default|GetAmmo) 1.0)))
            (Development|PrintString (Utilities|String|ToString(Float) _output_get)))))
      (else
        (goto _label Reset)))))

(event Custom|Stats
  (params (IsLethal :type Boolean) (Damage :type Float%20%28single-precision%29) (Ammo :type Float%20%28single-precision%29) (Range :type Float%20%28single-precision%29))
  ;[1 1 1] Weapon Stats
  (Variables|Default|SetIsLethal? IsLethal)
  (Variables|Default|SetDamage Damage)
  (Variables|Default|SetAmmo Ammo)
  (Variables|Default|SetRange Range))

(event Collision|EventActorBeginOverlap
  (params (OtherActor :type Actor%20Object%20Reference)))

(fn ConstructionScript)